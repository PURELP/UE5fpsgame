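; First-person shooter player pawn with movement, aim, weapon and health, plus a 20-second survival win and a death game-over.
; Enhanced Input sets intent flags; each Tick derives an Idle/Walk/Run/Aim state driving walk speed, while look sensitivity also follows it.
; Aiming interpolates FOV, with a looping timer restoring it on release.
; BeginPlay spawns a weapon attached to the control-rotated arm and creates HUD widgets; fire and reload forward to that weapon.
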(event Custom|outFOV
  (bind _camera (Variables|Default|GetCamera))
  (bind _fieldofview (Variables|/Script/Engine.CameraComponent|GetFieldOfView _camera))
  (Camera|SetFieldOfView _camera (Math|Interpolation|FInterpTo _fieldofview (Variables|Default|GetdefaultFOV) (Utilities|Time|GetWorldDeltaSeconds) 8.0))
  (if (Math|Float|NearlyEqual(Float) _fieldofview (Variables|Default|GetdefaultFOV) 0.5)
    (Utilities|Time|ClearandInvalidateTimerbyHandle (Variables|Default|GetoutFOVhandle))))

(event Input|EnhancedActionEvents|EnhancedInputActionIA_move
  (params (ActionValue :type Vector%202D%20Structure) (ElapsedSeconds :type Float%20%28double-precision%29) (TriggeredSeconds :type Float%20%28double-precision%29) (InputAction :type Input%20Action%20Object%20Reference :default "/Game/code/player/system/input/IA_move.IA_move"))
  (bind (_x _y) (Math|Vector2D|BreakVector2D ActionValue))
  (:Triggered
    (bind _output_get (Variables|Default|Setmove%20x _x))
    (Pawn|Input|AddMovementInput (Math|Vector|GetForwardVector (Math|Rotator|MakeRotator 0.0 0.0 (.yaw (Pawn|GetControlRotation :!class /Script/Engine.Pawn)))) _output_get false)
    (bind _output_get_2 (Variables|Default|Setmove%20y _y))
    (Pawn|Input|AddMovementInput (Math|Vector|GetRightVector (Math|Rotator|MakeRotator 0.0 0.0 (.yaw (Pawn|GetControlRotation :!class /Script/Engine.Pawn)))) _output_get_2 false))
  (:Completed
    (Variables|Default|Setmove%20x 0.0)
    (Variables|Default|Setmove%20y 0.0)))

(event Input|EnhancedActionEvents|EnhancedInputActionIA_look
  (params (ActionValue :type Vector%202D%20Structure) (ElapsedSeconds :type Float%20%28double-precision%29) (TriggeredSeconds :type Float%20%28double-precision%29) (InputAction :type Input%20Action%20Object%20Reference :default "/Game/code/player/system/input/IA_look.IA_look"))
  (bind (_x _y) (Math|Vector2D|BreakVector2D ActionValue))
  (Pawn|Input|AddControllerYawInput (* _x (CallFunction|Updatescopesensitivity) (Variables|Default|Getmousesensitivity)))
  (Pawn|Input|AddControllerPitchInput (* (* _y -1.0) (CallFunction|Updatescopesensitivity) (Variables|Default|Getmousesensitivity))))

(event Input|EnhancedActionEvents|EnhancedInputActionIA_run
  (params (ActionValue :type Boolean) (ElapsedSeconds :type Float%20%28double-precision%29) (TriggeredSeconds :type Float%20%28double-precision%29) (InputAction :type Input%20Action%20Object%20Reference :default "/Game/code/player/system/input/IA_run.IA_run"))
  (:Triggered
    (Variables|Default|Setwant%20to%20run true))
  (:Completed
    (Variables|Default|Setwant%20to%20run false)))

(event Input|EnhancedActionEvents|EnhancedInputActionIA_aim
  (params (ActionValue :type Boolean) (ElapsedSeconds :type Float%20%28double-precision%29) (TriggeredSeconds :type Float%20%28double-precision%29) (InputAction :type Input%20Action%20Object%20Reference :default "/Game/code/player/system/input/IA_aim.IA_aim"))
  (bind _camera (Variables|Default|GetCamera))
  (:Triggered
    (Variables|Default|Setwant%20to%20aim true)
    (Camera|SetFieldOfView _camera (Math|Interpolation|FInterpTo (Variables|/Script/Engine.CameraComponent|GetFieldOfView _camera) 75.0 (Utilities|Time|GetWorldDeltaSeconds) 8.0))
    (Utilities|Time|ClearandInvalidateTimerbyHandle (Variables|Default|GetoutFOVhandle)))
  (:Completed
    (Variables|Default|Setwant%20to%20aim false)
    (bind _returnvalue (Utilities|Time|SetTimerbyEvent (delegate Custom|outFOV) (Utilities|Time|GetWorldDeltaSeconds) true))
    (Variables|Default|SetoutFOVhandle _returnvalue)))

(event Input|EnhancedActionEvents|EnhancedInputActionIA-fire
  (params (ActionValue :type Boolean) (ElapsedSeconds :type Float%20%28double-precision%29) (TriggeredSeconds :type Float%20%28double-precision%29) (InputAction :type Input%20Action%20Object%20Reference :default "/Game/code/player/system/input/IA-fire.IA-fire"))
  (:Started
    (if (not (Variables|Default|Getisfiring))
      (if (not (Variables|Default|Getisdead))
        (if (Utilities|Enum|NotEqual(Enum) (Variables|Default|GetE_playerstate) "NewEnumerator2")
          (Class|BI-fire|Startweaponfire(Message) (Variables|Default|Getcurrentweapon) self)))))
  (:Completed
    (Default|Stopfire (Variables|Default|Getcurrentweapon))
    (Variables|Default|Setisfiring false)))

(event Input|EnhancedActionEvents|EnhancedInputActionIA-reload
  (params (ActionValue :type Boolean) (ElapsedSeconds :type Float%20%28double-precision%29) (TriggeredSeconds :type Float%20%28double-precision%29) (InputAction :type Input%20Action%20Object%20Reference :default "/Game/code/player/system/input/IA-reload.IA-reload"))
  (:Started
    (Default|Reload (Variables|Default|Getcurrentweapon) self)))

(event EventBeginPlay
  (Utilities|FlowControl|Sequence
    (:then_0
      (bind _as玩家控制器 (Utilities|Casting|CastToPlayerController (Pawn|GetController)))
      (Input|AddMappingContext (PlayerController|LocalPlayerSubsystems|GetEnhancedInputLocalPlayerSubsystem _as玩家控制器) "/Game/code/player/system/input/IMC_fpsinput.IMC_fpsinput" 0 "(bIgnoreAllPressedKeysUntilRelease=True,bForceImmediately=False,bNotifyUserSettings=False)")
      (CallFunction|Spawnweapon "/Game/code/weapon/BP-virtus.BP-virtus_C")
      (CallFunction|UpdatedefaultFOV)
      (bind _returnvalue (UserInterface|CreateWidget "/Game/code/UI/UI-mainui.UI-mainui_C"))
      (bind _output_get (Variables|Default|Setmainui _returnvalue))
      (UserInterface|Viewport|AddtoViewport _output_get 0))
    (:then_1
      (bind _returnvalue_2 (UserInterface|CreateWidget "/Game/code/UI/blood-UI.blood-UI_C"))
      (bind _output_get_2 (Variables|Default|SetUIblood _returnvalue_2))
      (UserInterface|Viewport|AddtoViewport _output_get_2 0))
    (:then_2
      (bind _returnvalue_3 (UserInterface|CreateWidget "/Game/code/UI/countdown-UI.countdown-UI_C"))
      (bind _output_get_3 (Variables|Default|SetUIcount _returnvalue_3))
      (UserInterface|Viewport|AddtoViewport _output_get_3 0))))

(event Game|Damage|EventAnyDamage
  (params (Damage :type Float%20%28single-precision%29) (DamageType :type Damage%20Type%20Object%20Reference) (InstigatedBy :type Controller%20Object%20Reference) (DamageCauser :type Actor%20Object%20Reference))
  (Variables|Default|Setplayerblood (Math|Float|Clamp(Float) (- (Variables|Default|Getplayerblood) Damage) 0.0 (- (Variables|Default|Getplayerblood) Damage)))
  (if (<= (Variables|Default|Getplayerblood) 0.0)
    (bind _returnvalue (UserInterface|CreateWidget "/Game/code/UI/gameover-UI.gameover-UI_C"))
    (UserInterface|Viewport|AddtoViewport _returnvalue 0)
    (Widget|RemovefromParent (Variables|Default|GetUIcount))
    (Widget|RemovefromParent (Variables|Default|GetUIblood))
    (Input|DisableInput 0)))

(event EventTick
  (params (DeltaSeconds :type Float%20%28single-precision%29))
  (bind _returnvalue (Pawn|GetControlRotation :!class /Script/Engine.Pawn))
  (Transformation|SetWorldRotation (Variables|Default|Getarm) (Math|Rotator|MakeRotator 0.0 (.pitch _returnvalue) (.yaw _returnvalue)) false false)
  (CallFunction|Updateplayerstate)
  (CallFunction|Updatemovespeed)
  (Development|PrintString (Utilities|String|ToString(Float) (Variables|/Script/Engine.CharacterMovementComponent|GetMaxWalkSpeed (Variables|Character|GetCharacterMovement))) true true "(R=0.000000,G=0.660000,B=1.000000,A=1.000000)" 0.0)
  (if (<= (- 2e+01 (Utilities|Time|GetGameTimeinSeconds)) 0.0)
    (Utilities|FlowControl|DoOnce false
      (:Completed
        (if (> (Variables|Default|Getplayerblood) 0.0)
          (bind _returnvalue_2 (UserInterface|CreateWidget "/Game/code/UI/win-UI.win-UI_C"))
          (UserInterface|Viewport|AddtoViewport _returnvalue_2 0)
          (Widget|RemovefromParent (Variables|Default|GetUIcount))
          (Widget|RemovefromParent (Variables|Default|GetUIblood)))))))

(fn ConstructionScript)

(fn Updateplayerstate
  (if (Variables|Default|Getwant%20to%20aim)
    (Variables|Default|SetE_playerstate "NewEnumerator3")
    (elif (> (Variables|Default|Getmove%20x) 0.0)
      (if (Variables|Default|Getwant%20to%20run)
        (Variables|Default|SetE_playerstate "NewEnumerator2")
        (else
          (Variables|Default|SetE_playerstate "NewEnumerator1")))
      (elif (> (Math|Vector|VectorLength (Variables|/Script/Engine.MovementComponent|GetVelocity (Variables|Character|GetCharacterMovement))) 0.0)
        (Variables|Default|SetE_playerstate "NewEnumerator1")
        (else
          (Variables|Default|SetE_playerstate "NewEnumerator0"))))))

(fn Updatemovespeed
  (Variables|/Script/Engine.CharacterMovementComponent|SetMaxWalkSpeed (Variables|Character|GetCharacterMovement) (Utilities|Select :Index (Variables|Default|GetE_playerstate) :NewEnumerator0 4e+02 :NewEnumerator1 4e+02 :NewEnumerator2 6e+02 :NewEnumerator3 265.0)))

(fn Spawnweapon
  (params (Class :type Actor%20Class%20Reference))
  (bind _returnvalue (Game|SpawnActorfromClass Class (Math|Transform|MakeTransform "0, 0, 0" "0, 0, 0" "1.000000,1.000000,1.000000") "Undefined" "MultiplyWithRoot" self 0))
  (bind _asbp_weaponbase (Utilities|Casting|CastToBP-weaponbase _returnvalue))
  (bind _output_get (Variables|Default|Setcurrentweapon _asbp_weaponbase))
  (Transformation|AttachComponentToComponent _output_get (Variables|Default|Getarm) "None" "KeepRelative" "KeepRelative" "KeepRelative" true))

(fn UpdatedefaultFOV
  (Variables|Default|SetdefaultFOV (Variables|/Script/Engine.CameraComponent|GetFieldOfView (Variables|Default|GetCamera))))

(fn Updatescopesensitivity
  (return (Utilities|Select :Index (Variables|Default|GetE_playerstate) :NewEnumerator0 1.0 :NewEnumerator1 1.0 :NewEnumerator2 1.0 :NewEnumerator3 0.6)))